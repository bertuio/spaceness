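; Artifact spawner actor: each Spawn_Artefacts call spawns the next ArtifMass class at a random point in a box set by Point's location and scale, with a random EndPosition.
; ArtifMass works as a shuffle bag, reshuffled after each full pass.
; The array fill and looping timer are disconnected, and BeginPlay is empty.
; ChooseArtif offers an uncalled weighted pick from ArtifCl, while ShuffleArtif's fill loops are empty ranges.
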(event Custom|Spawn_Artefacts
  (bind _point (Variables|Default|Getpoint))
  ;[0.7791 1 0.8103] SPAWN_ARTEFACTS
  (Game|SpawnActorfromClass (Utilities|Array|Get(acopy) (Variables|Default|Getartif_mass) (Variables|Default|GetIterator)) (Math|Transform|MakeTransform (Math|Random|RandomPointinBoundingBox (Transformation|GetWorldLocation _point) (Transformation|GetWorldScale _point)) "0, 0, 0" "1,1,1") "Undefined" 0 (Utilities|Array|Get(acopy) (Variables|Default|Getend_position) (Math|Random|RandomInteger 5)) 0)
  (bind _result (Math|Integer|IncrementInt (Variables|Default|GetIterator))
    (:%20%20
      (if (>= _result (Utilities|Array|Length (Variables|Default|Getartif_mass)))
        (Variables|Default|SetIterator 0)
        (Utilities|Array|Shuffle (Variables|Default|Getartif_mass))))))

(event EventBeginPlay)

(fn ConstructionScript)

(fn ChooseArtif
  (Variables|Default|SetMaxRand 0.0)
  (Variables|Default|SetCurRand 0.0)
  (Variables|Default|SetCurMin 0.0)
  (for _array_element (Variables|Default|Getartif_cl)
    (Variables|Default|SetMaxRand (+ (.chance (Utilities|Struct|Breakartif_structure _array_element)) (Variables|Default|GetMaxRand))))
  (Variables|Default|SetCurRand (Math|Random|RandomFloatinRange 0.0 (Variables|Default|GetMaxRand)))
  (for _array_element_2 (Variables|Default|Getartif_cl)
    (if (< (Variables|Default|GetCurRand) (+ (.chance (Utilities|Struct|Breakartif_structure _array_element_2)) (Variables|Default|GetCurMin)))
      (return (.type (Utilities|Struct|Breakartif_structure _array_element_2)))
      (else
        (Variables|Default|SetCurMin (+ (.chance (Utilities|Struct|Breakartif_structure _array_element_2)) (Variables|Default|GetCurMin)))))))

(fn ShuffleArtif
  (for _index (range 1 0)
    (Utilities|Array|Add (Variables|Default|Getartif_mass) 0))
  (for _index_2 (range 1 0)
    (Utilities|Array|Add (Variables|Default|Getartif_mass) 0))
  (for _index_3 (range 1 0)
    (Utilities|Array|Add (Variables|Default|Getartif_mass) 0))
  (for _index_4 (range 1 0)
    (Utilities|Array|Add (Variables|Default|Getartif_mass) 0))
  (for _index_5 (range 1 0)
    (Utilities|Array|Add (Variables|Default|Getartif_mass) 0))
  (Utilities|Array|Shuffle (Variables|Default|Getartif_mass)))