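; Actor Blueprint that moves a list of actors along orbits as game time passes, as part of SimpleOM.
; While SOM is enabled, Tick passes time since creation to UpdateAllActors, which updates each entry's position.
; The construction script places all actors at time zero for editor preview.
; Optional debug drawing, in editor or at BeginPlay, rebuilds instanced orbit-plane meshes from each entry converted to SOM data.
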(event Custom|UpdateAllActors
  (params (New%20Time :type Float%20%28single-precision%29))
  (for _array_element (Variables|Default|GetActors)
    (CallFunction|UpdateActorPosition _array_element New%20Time)))

(event EventBeginPlay
  (|CallParentFunction)
  (if (Variables|Default|GetEnable%20Debug%20Orbits)
    (CallFunction|DrawDebugOrbits)))

(event Collision|EventActorBeginOverlap
  (params (OtherActor :type Actor%20Object%20Reference))
  (|CallParentFunction OtherActor))

(event EventTick
  (params (DeltaSeconds :type Float%20%28single-precision%29))
  (|CallParentFunction DeltaSeconds)
  (if (Variables|Default|GetEnable%20SOM)
    (CallFunction|UpdateAllActors (Actor|GetGameTimeSinceCreation))))

(fn ConstructionScript
  (|CallParentFunction)
  (CallFunction|UpdateAllActors 0.0)
  (if (Variables|Default|GetShow%20Debug%20Orbits%20in%20Editor)
    (CallFunction|DrawDebugOrbits)))

(fn DrawDebugOrbits
  (Components|InstancedStaticMesh|ClearInstances (Variables|Default|GetOverflowOrbitInstancedMeshes))
  (for _index (range 0 (- (Utilities|Array|Length (Variables|Default|GetActors)) 1))
    (CallFunction|AddOrbitPlaneInstance _index (CallFunction|ConvertActorDatatoSOMData (Utilities|Array|Get(acopy) (Variables|Default|GetActors) _index)))))